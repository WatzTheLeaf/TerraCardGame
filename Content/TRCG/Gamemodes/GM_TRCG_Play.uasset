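; Play game mode for TRCG that bootstraps the gameplay managers and requests the game HUD.
; InitGamemodeDispatchers binds the ready dispatchers, forming an event-driven startup chain instead of spawning everything at once.
; HUD ready spawns the card manager and asks HUD_TRCG to create the game HUD.
; Card manager ready spawns the tile manager with a fixed-size grid, whose ready event spawns the planet stats manager.
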(event Custom|OnHUDReadyEvent
  (Game|SpawnActorfromClass "/Game/TRCG/Managers/BP_TRCG_CardManager.BP_TRCG_CardManager_C" (Math|Transform|MakeTransform "0, 0, 0") "Undefined" "MultiplyWithRoot" 0 0)
  (bind _ashud_trcg (Utilities|Casting|CastToHUD_TRCG (HUD|GetHUD (Game|GetPlayerController 0))))
  (Default|CallCreateGameHUDRequest _ashud_trcg))

(event Custom|OnCardManagerReadyEvent
  (Game|SpawnActorfromClass "/Game/TRCG/Managers/BP_TRCG_TileManager.BP_TRCG_TileManager_C" (Math|Transform|MakeTransform "0, 0, 0") "Undefined" "MultiplyWithRoot" 0 4 6 0))

(event Custom|OnTileManagerReadyEvent
  (Game|SpawnActorfromClass "/Game/TRCG/Managers/BP_TRCG_PlanetStatsManager.BP_TRCG_PlanetStatsManager_C" (Math|Transform|MakeTransform "0, 0, 0") "Undefined" "MultiplyWithRoot" 0 0))

(event EventInitGamemodeDispatchers
  (EventDispatchers|BindEventtoOnCardManagerReady (delegate Custom|OnCardManagerReadyEvent))
  (EventDispatchers|BindEventtoOnTileManagerReady (delegate Custom|OnTileManagerReadyEvent))
  (EventDispatchers|BindEventtoOnHUDReady (delegate Custom|OnHUDReadyEvent)))

(fn ConstructionScript)