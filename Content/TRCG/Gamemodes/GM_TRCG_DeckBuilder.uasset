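; Game mode for the TRCG deck builder that sets up the menu, player view and card display.
; InitGamemodeDispatchers binds a handler to the HUD-ready event, so setup waits for the HUD.
; The handler asks HUD_TRCG to create the menu widget, teleports the player pawn to a fixed raised transform, and spawns BP_TRCG_DisplayCardManager configured with a three-column layout.
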(event Custom|OnHUDReadyEvent
  (bind _ashud_trcg (Utilities|Casting|CastToHUD_TRCG (HUD|GetHUD (Game|GetPlayerController 0))))
  (Default|CallCreateMenuWidgetRequest _ashud_trcg)
  (Transformation|SetActorTransform (Game|Player|GetPlayerPawn 0) (Math|Transform|MakeTransform "0.000000,0.000000,300.000000" "-90.000000,180.000000,180.000000") false true)
  (Game|SpawnActorfromClass "/Game/TRCG/Gameplay/Cards/Display/BP_TRCG_DisplayCardManager.BP_TRCG_DisplayCardManager_C" (Math|Transform|MakeTransform "0.000000,0.000000,100.000000") "Undefined" "MultiplyWithRoot" 0 1.5e+02 2e+02 "0.000000,0.000000,100.000000" 3 0))

(event EventInitGamemodeDispatchers
  (EventDispatchers|BindEventtoOnHUDReady (delegate Custom|OnHUDReadyEvent)))

(fn ConstructionScript)