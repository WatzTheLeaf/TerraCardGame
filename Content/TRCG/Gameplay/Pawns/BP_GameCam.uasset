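; BP_GameCam is the player camera pawn for a tile-based card game, handling view control and card play.
; Enhanced Input pans relative to arm yaw, rotates, and sets a clamped zoom length that Tick smooths.
; Interacting plays the active card on the tile under the cursor, while a looping timer sends that card's effect preview to StatManager.
; It also coordinates startup with the game mode, HUD and TileManager.
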(event Custom|OnReadyToCreateHUDEvent
  (bind _ashud_trcg (Utilities|Casting|CastToHUD_TRCG (HUD|GetHUD (Game|GetPlayerController 0))))
  (Default|CallCreateGameHUDRequest _ashud_trcg)
  (bind _asbp_trcg_tile_manager (Utilities|Casting|CastToBP_TRCG_TileManager (Variables|/Script/TerraCardGame.TrcgGameInstance|GetTileManager (Class|TrcgPawn|GetTrcgGameInstance))))
  (Default|CallOnPlayerReady _asbp_trcg_tile_manager))

(event Input|EnhancedActionEvents|EnhancedInputActionIA_TrcgInteract
  (params (ActionValue :type Boolean) (ElapsedSeconds :type Float%20%28double-precision%29) (TriggeredSeconds :type Float%20%28double-precision%29) (InputAction :type Input%20Action%20Object%20Reference :default "/Game/TRCG/Controls/IA_TrcgInteract.IA_TrcgInteract"))
  (bind _returnvalue (Game|GetPlayerController 0))
  (bind _hitresult (Game|Player|GetHitResultUnderCursorbyChannel _returnvalue "TraceTypeQuery1" false))
  (bind _hitactor (Collision|BreakHitResult _hitresult))
  (:Started
    (Utilities|IsValid _hitactor
      (:Is%20Valid
        (bind _asbp_trcg_tile (Utilities|Casting|CastToBP_TRCG_Tile _hitactor))
        (bind _asgi_trcg (Utilities|Casting|CastToGI_TRCG (Class|TrcgPawn|GetTrcgGameInstance)))
        (Default|PlayActiveCardfromHand (Variables|/Game/TRCG/General/GI_TRCG.GI_TRCG_C|GetCardManager _asgi_trcg) _asbp_trcg_tile)))))

(event Input|EnhancedActionEvents|EnhancedInputActionIA_TrcgZoom
  (params (ActionValue :type Float%20%28double-precision%29) (ElapsedSeconds :type Float%20%28double-precision%29) (TriggeredSeconds :type Float%20%28double-precision%29) (InputAction :type Input%20Action%20Object%20Reference :default "/Game/TRCG/Controls/IA_TrcgZoom.IA_TrcgZoom"))
  (Variables|Default|SetArmTargetLen (Math|Float|Clamp(Float) (+ (Variables|Default|GetArmTargetLen) (* ActionValue 75.0)) 3e+02 (Variables|Default|GetMaxArmLenght))))

(event Input|EnhancedActionEvents|EnhancedInputActionIA_TrcgMove
  (params (ActionValue :type Vector%202D%20Structure) (ElapsedSeconds :type Float%20%28double-precision%29) (TriggeredSeconds :type Float%20%28double-precision%29) (InputAction :type Input%20Action%20Object%20Reference :default "/Game/TRCG/Controls/IA_TrcgMove.IA_TrcgMove"))
  (bind _arm (Variables|Default|GetArm))
  (bind _relativerotation (Variables|/Script/Engine.SceneComponent|GetRelativeRotation _arm))
  (bind _returnvalue (Math|Rotator|MakeRotator 0.0 0.0 (.yaw _relativerotation)))
  (Class|PawnMovementComponent|AddInputVector (Variables|Default|GetMovementComponent) (+ (* (Math|Vector|GetRightVector _returnvalue) (.x ActionValue)) (* (.y ActionValue) (Math|Vector|GetForwardVector _returnvalue))) false))

(event Input|EnhancedActionEvents|EnhancedInputActionIA_TrcgTurn
  (params (ActionValue :type Float%20%28double-precision%29) (ElapsedSeconds :type Float%20%28double-precision%29) (TriggeredSeconds :type Float%20%28double-precision%29) (InputAction :type Input%20Action%20Object%20Reference :default "/Game/TRCG/Controls/IA_TrcgTurn.IA_TrcgTurn"))
  (Transformation|AddRelativeRotation (Variables|Default|GetArm) (Math|Rotator|MakeRotator 0.0 0.0 (* ActionValue (Variables|Default|GetRotationSpeed) (Utilities|Time|GetWorldDeltaSeconds))) false false))

(event EventTick
  (params (DeltaSeconds :type Float%20%28single-precision%29))
  (bind _arm (Variables|Default|GetArm))
  (Variables|/Script/Engine.SpringArmComponent|SetTargetArmLength _arm (Math|Interpolation|FInterpTo (Variables|/Script/Engine.SpringArmComponent|GetTargetArmLength _arm) (Variables|Default|GetArmTargetLen) DeltaSeconds 1e+01)))

(event EventPossessed
  (params (NewController :type Controller%20Object%20Reference))
  (Input|AddMappingContext (PlayerController|LocalPlayerSubsystems|GetEnhancedInputLocalPlayerSubsystem (Game|GetPlayerController 0)) "/Game/TRCG/Controls/IMC_TRCG_Game.IMC_TRCG_Game" 0 "(bIgnoreAllPressedKeysUntilRelease=True,bForceImmediately=False,bNotifyUserSettings=False)")
  (Utilities|Time|SetTimerbyFunctionName 0 "Evaluate" 0.2 true true 1.0))

(event EventBeginPlay
  (EventDispatchers|BindEventtoOnReadytoCreateHUD (delegate Custom|OnReadyToCreateHUDEvent))
  (bind _asgm_trcg_play (Utilities|Casting|CastToGM_TRCG_Play (Game|GetGameMode)))
  (Default|CallOnPlayerPawnReady _asgm_trcg_play))

(fn ConstructionScript)

(fn Evaluate
  (bind _returnvalue (Game|GetPlayerController 0))
  (bind _returnvalue_2 (Class|TrcgPawn|GetTrcgGameInstance))
  (bind _returnvalue_3 (Class|TrcgPawn|GetTrcgGameInstance))
  (bind _hitresult (Game|Player|GetHitResultUnderCursorbyChannel _returnvalue "TraceTypeQuery1" false))
  (bind _statmanager (Variables|/Script/TerraCardGame.TrcgGameInstance|GetStatManager _returnvalue_3))
  (bind _hitactor (Collision|BreakHitResult _hitresult))
  (bind _asgi_trcg (Utilities|Casting|CastToGI_TRCG _returnvalue_2))
  (if (Default|HasActiveCard (Variables|/Game/TRCG/General/GI_TRCG.GI_TRCG_C|GetCardManager _asgi_trcg))
    (Utilities|IsValid _hitactor
      (:Is%20Valid
        (bind _asbp_trcg_tile (Utilities|Casting|CastToBP_TRCG_Tile _hitactor)
          (:then
            (if (Default|CanbePlayedon (Variables|/Game/TRCG/General/GI_TRCG.GI_TRCG_C|GetCardManager _asgi_trcg) _asbp_trcg_tile (Default|GetActiveCard (Variables|/Game/TRCG/General/GI_TRCG.GI_TRCG_C|GetCardManager _asgi_trcg)))
              (bind _returnvalue_4 (Game|ConstructObjectfromClass (Variables|/Script/TerraCardGame.TrcgCardData|GetCardEffect (Variables|/Game/TRCG/Gameplay/Cards/Base/BP_TRCG_Card.BP_TRCG_Card_C|GetData (Default|GetActiveCard (Variables|/Game/TRCG/General/GI_TRCG.GI_TRCG_C|GetCardManager _asgi_trcg))))))
              (bind _returnvalue_5 (Class|TrcgCardEffect|PreviewEffect _returnvalue_4 (Utilities|Array|FindItem (Variables|/Script/TerraCardGame.TrcgTileManager|GetTiles (Variables|/Script/TerraCardGame.TrcgGameInstance|GetTileManager _returnvalue_2)) _asbp_trcg_tile)))
              (Variables|/Script/TerraCardGame.TrcgPlanetStatsManager|SetPreview _statmanager _returnvalue_5)
              (else
                (Utilities|Map|Clear (Variables|/Script/TerraCardGame.TrcgPlanetStatsManager|GetPreview _statmanager) :!label _label))))
          (:CastFailed
            (goto _label))))
      (:Is%20Not%20Valid
        (goto _label)))
    (else
      (goto _label))))