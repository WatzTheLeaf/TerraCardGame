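; Tile manager for TRCG that builds the world's tile grid and bounds the play area.
; On BeginPlay it registers with the game instance, generates a grid tagged raw and neutral, then notifies the GameSpawnManager that it is ready.
; When the player is ready, it teleports the pawn to the grid center and spawns a blocking volume there, sized from the grid dimensions at 150 units per tile plus a margin.
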(event Custom|OnPlayerReadyEvent
  (CallFunction|GenerateLimit))

(event EventBeginPlay
  (EventDispatchers|BindEventtoOnPlayerReady (delegate Custom|OnPlayerReadyEvent))
  (Variables|/Script/TerraCardGame.TrcgGameInstance|SetTileManager (Class|TrcgActor|GetTrcgGameInstance) self)
  (Class|TrcgTileManager|GenerateGrid (Utilities|Set|MakeSet "(TagName=\"Tiles.State.Raw\")" "(TagName=\"Tiles.Type.Neutral\")"))
  (bind _asgi_trcg (Utilities|Casting|CastToGI_TRCG (Class|TrcgActor|GetTrcgGameInstance)))
  (Default|CallOnTileManagerReady (Variables|/Game/TRCG/General/GI_TRCG.GI_TRCG_C|GetGameSpawnManager _asgi_trcg)))

(fn ConstructionScript)

(fn GenerateLimit
  (bind _returnvalue (Game|Player|GetPlayerPawn 0))
  (bind _gridxsize (Variables|Default|GetGridXSize))
  (bind _gridysize (Variables|Default|GetGridYSize))
  (bind _returnvalue_2 (* 1.5e+02 _gridxsize))
  (bind _returnvalue_3 (* _gridysize 1.5e+02))
  (bind _returnvalue_4 (/ _returnvalue_3 2.0))
  (bind _returnvalue_5 (/ _returnvalue_2 2.0))
  (Transformation|Teleport _returnvalue (Math|Vector|MakeVector _returnvalue_5 _returnvalue_4 (.z (Transformation|GetActorLocation _returnvalue))) (Transformation|GetActorRotation _returnvalue))
  (Game|SpawnActorfromClass "/Game/TRCG/Gameplay/Misc/BP_TRCG_BlockingVolume.BP_TRCG_BlockingVolume_C" (Math|Transform|MakeTransform (Math|Vector|MakeVector _returnvalue_5 _returnvalue_4 0.0)) "Undefined" "MultiplyWithRoot" 0 (Math|Vector2D|MakeVector2D (+ _returnvalue_4 5e+01) (+ _returnvalue_5 5e+01)) 0)
  (return))