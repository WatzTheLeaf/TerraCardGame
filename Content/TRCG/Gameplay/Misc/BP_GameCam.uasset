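; BP_GameCam is the player-controlled gameplay camera for TRCG, with move, turn and zoom on Enhanced Input.
; BeginPlay adds the game mapping context, creates the HUD widget and shows the mouse cursor.
; Movement follows the spring arm's yaw, so panning stays relative to the view, while turn input rotates the arm.
; Zoom adjusts a clamped target arm length, which Tick smoothly interpolates toward.
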(event Input|EnhancedActionEvents|EnhancedInputActionIA_TrcgZoom
  (params (ActionValue :type Float%20%28double-precision%29) (ElapsedSeconds :type Float%20%28double-precision%29) (TriggeredSeconds :type Float%20%28double-precision%29) (InputAction :type Input%20Action%20Object%20Reference :default "/Game/TRCG/Controls/IA_TrcgZoom.IA_TrcgZoom"))
  (Variables|Default|SetArmTargetLen (Math|Float|Clamp(Float) (+ (Variables|Default|GetArmTargetLen) (* ActionValue 75.0)) 3e+02 (Variables|Default|GetMaxArmLenght))))

(event Input|EnhancedActionEvents|EnhancedInputActionIA_TrcgMove
  (params (ActionValue :type Vector%202D%20Structure) (ElapsedSeconds :type Float%20%28double-precision%29) (TriggeredSeconds :type Float%20%28double-precision%29) (InputAction :type Input%20Action%20Object%20Reference :default "/Game/TRCG/Controls/IA_TrcgMove.IA_TrcgMove"))
  (bind _arm (Variables|Default|GetArm))
  (bind _relativerotation (Variables|/Script/Engine.SceneComponent|GetRelativeRotation _arm))
  (bind _returnvalue (Math|Rotator|MakeRotator 0.0 0.0 (.yaw _relativerotation)))
  (Class|PawnMovementComponent|AddInputVector (Variables|Default|GetMovementComponent) (+ (* (Math|Vector|GetRightVector _returnvalue) (.x ActionValue)) (* (.y ActionValue) (Math|Vector|GetForwardVector _returnvalue))) false))

(event Input|EnhancedActionEvents|EnhancedInputActionIA_TrcgTurn
  (params (ActionValue :type Float%20%28double-precision%29) (ElapsedSeconds :type Float%20%28double-precision%29) (TriggeredSeconds :type Float%20%28double-precision%29) (InputAction :type Input%20Action%20Object%20Reference :default "/Game/TRCG/Controls/IA_TrcgTurn.IA_TrcgTurn"))
  (Transformation|AddRelativeRotation (Variables|Default|GetArm) (Math|Rotator|MakeRotator 0.0 0.0 (* ActionValue (Variables|Default|GetRotationSpeed))) false false))

(event EventTick
  (params (DeltaSeconds :type Float%20%28single-precision%29))
  (bind _arm (Variables|Default|GetArm))
  (Variables|/Script/Engine.SpringArmComponent|SetTargetArmLength _arm (Math|Interpolation|FInterpTo (Variables|/Script/Engine.SpringArmComponent|GetTargetArmLength _arm) (Variables|Default|GetArmTargetLen) DeltaSeconds 1e+01)))

(event EventBeginPlay
  (bind _returnvalue (Game|GetPlayerController 0))
  (Input|AddMappingContext (PlayerController|LocalPlayerSubsystems|GetEnhancedInputLocalPlayerSubsystem (Game|GetPlayerController 0)) "/Game/TRCG/Controls/IMC_TRCG_Game.IMC_TRCG_Game" 0 "(bIgnoreAllPressedKeysUntilRelease=True,bForceImmediately=False,bNotifyUserSettings=False)")
  (bind _returnvalue_2 (UserInterface|CreateWidget "/Game/TRCG/HUD/WBP_GameHUD.WBP_GameHUD_C" _returnvalue))
  (UserInterface|Viewport|AddtoViewport _returnvalue_2 0)
  (Variables|/Script/Engine.PlayerController|SetbShowMouseCursor _returnvalue true))

(fn ConstructionScript)