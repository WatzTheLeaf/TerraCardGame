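; BP_TRCG_BlockingVolume is a resizable rectangular boundary made of four thin, very tall box volumes, apparently meant to block movement around an area.
; The construction script uses the Size variable to stretch the UP, DOWN, LEFT and RIGHT boxes and offset them to the rectangle's edges, with Size.Y as the X half-extent and Size.X as the Y half-extent.
; It has no runtime logic, as BeginPlay is empty.
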(event EventBeginPlay)

(fn ConstructionScript
  (Components|Box|SetBoxExtent (Variables|Default|GetVolumeUP) (Math|Vector|MakeVector 5.0 (.x (Variables|Default|GetSize)) 1e+04) true)
  (Components|Box|SetBoxExtent (Variables|Default|GetVolumeDOWN) (Math|Vector|MakeVector 5.0 (.x (Variables|Default|GetSize)) 1e+04) true)
  (Components|Box|SetBoxExtent (Variables|Default|GetVolumeLEFT) (Math|Vector|MakeVector (.y (Variables|Default|GetSize)) 5.0 1e+04) true)
  (Components|Box|SetBoxExtent (Variables|Default|GetVolumeRIGHT) (Math|Vector|MakeVector (.y (Variables|Default|GetSize)) 5.0 1e+04) true)
  (Transformation|SetRelativeLocation (Variables|Default|GetVolumeUP) (Math|Vector|MakeVector (.y (Variables|Default|GetSize)) 0.0 0.0) false true)
  (Transformation|SetRelativeLocation (Variables|Default|GetVolumeDOWN) (Math|Vector|MakeVector (- 0.0 (.y (Variables|Default|GetSize))) 0.0 0.0) false true)
  (Transformation|SetRelativeLocation (Variables|Default|GetVolumeLEFT) (Math|Vector|MakeVector 0.0 (- 0.0 (.x (Variables|Default|GetSize))) 0.0) false true)
  (Transformation|SetRelativeLocation (Variables|Default|GetVolumeRIGHT) (Math|Vector|MakeVector 0.0 (.x (Variables|Default|GetSize)) 0.0) false true))