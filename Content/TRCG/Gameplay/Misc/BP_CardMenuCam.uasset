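; Deck-builder menu camera pawn that pans and zooms over display cards and lets the player add them to the deck.
; On BeginPlay it adds the menu input context, shows the deck-builder widget and cursor, and starts a looping cursor-trace timer.
; That trace feeds the hovered card's FocusAngle with the impact point.
; Clicking a card increments its count in the GameInstance's GlobalDeck unless full, then refreshes the widget's list.
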(event Input|EnhancedActionEvents|EnhancedInputActionIA_MoveMenu
  (params (ActionValue :type Vector%202D%20Structure) (ElapsedSeconds :type Float%20%28double-precision%29) (TriggeredSeconds :type Float%20%28double-precision%29) (InputAction :type Input%20Action%20Object%20Reference :default "/Game/TRCG/Controls/IA_MoveMenu.IA_MoveMenu"))
  (Class|PawnMovementComponent|AddInputVector (Variables|Default|GetMovementComponent) (Math|Vector|MakeVector (.x ActionValue) (.y ActionValue) 0.0) false))

(event Input|EnhancedActionEvents|EnhancedInputActionIA_ZoomMenu
  (params (ActionValue :type Float%20%28double-precision%29) (ElapsedSeconds :type Float%20%28double-precision%29) (TriggeredSeconds :type Float%20%28double-precision%29) (InputAction :type Input%20Action%20Object%20Reference :default "/Game/TRCG/Controls/IA_ZoomMenu.IA_ZoomMenu"))
  (bind _arm (Variables|Default|GetArm))
  (Variables|/Script/Engine.SpringArmComponent|SetTargetArmLength _arm (Math|Float|Clamp(Float) (+ (Variables|/Script/Engine.SpringArmComponent|GetTargetArmLength _arm) (* ActionValue 75.0)) 0.0 (Variables|Default|GetMaxArmLenght))))

(event Input|EnhancedActionEvents|EnhancedInputActionIA_MenuInteract
  (params (ActionValue :type Boolean) (ElapsedSeconds :type Float%20%28double-precision%29) (TriggeredSeconds :type Float%20%28double-precision%29) (InputAction :type Input%20Action%20Object%20Reference :default "/Game/TRCG/Controls/IA_MenuInteract.IA_MenuInteract"))
  (bind _returnvalue (Game|GetPlayerController 0))
  (bind _returnvalue_2 (Class|TrcgPawn|GetTrcgGameInstance))
  (bind _hitresult (Game|Player|GetHitResultUnderCursorbyChannel _returnvalue "TraceTypeQuery1" false))
  (bind _globaldeck (Variables|/Script/TerraCardGame.TrcgGameInstance|GetGlobalDeck _returnvalue_2))
  (bind _hitactor (Collision|BreakHitResult _hitresult))
  (:Started
    (if (not (Class|TrcgGameInstance|IsDeckFull (Class|TrcgPawn|GetTrcgGameInstance)))
      (Utilities|IsValid _hitactor
        (:Is%20Valid
          (bind _asbp_trcg_display_card (Utilities|Casting|CastToBP_TRCG_DisplayCard _hitactor))
          (if (.ReturnValue (Utilities|Map|Find _globaldeck (Variables|/Game/TRCG/Gameplay/Cards/Display/BP_TRCG_DisplayCard.BP_TRCG_DisplayCard_C|GetData _asbp_trcg_display_card)))
            (Utilities|Map|Add _globaldeck (Variables|/Game/TRCG/Gameplay/Cards/Display/BP_TRCG_DisplayCard.BP_TRCG_DisplayCard_C|GetData _asbp_trcg_display_card) (+ (.Value (Utilities|Map|Find _globaldeck (Variables|/Game/TRCG/Gameplay/Cards/Display/BP_TRCG_DisplayCard.BP_TRCG_DisplayCard_C|GetData _asbp_trcg_display_card))) 1))
            (else
              (Utilities|Map|Add _globaldeck (Variables|/Game/TRCG/Gameplay/Cards/Display/BP_TRCG_DisplayCard.BP_TRCG_DisplayCard_C|GetData _asbp_trcg_display_card) 1)))
          (Default|UpdateCardList (Variables|Default|GetDeckBuilderHUD)))))))

(event EventBeginPlay
  (bind _returnvalue (Game|GetPlayerController 0))
  (Input|AddMappingContext (PlayerController|LocalPlayerSubsystems|GetEnhancedInputLocalPlayerSubsystem (Game|GetPlayerController 0)) "/Game/TRCG/Controls/IMC_TRCG_Menu.IMC_TRCG_Menu" 0 "(bIgnoreAllPressedKeysUntilRelease=True,bForceImmediately=False,bNotifyUserSettings=False)")
  (Utilities|Time|SetTimerbyFunctionName 0 "CursorChanel" 0.1 true true)
  (bind _returnvalue_2 (UserInterface|CreateWidget "/Game/TRCG/HUD/WBP_DeckBuilder.WBP_DeckBuilder_C" _returnvalue))
  (UserInterface|Viewport|AddtoViewport _returnvalue_2 0)
  (Variables|/Script/Engine.PlayerController|SetbShowMouseCursor _returnvalue true)
  (bind _output_get (Variables|Default|SetDeckBuilderHUD _returnvalue_2))
  (Input|SetInputModeGameandUI _returnvalue _output_get "DoNotLock" false false))

(fn ConstructionScript)

(fn CursorChanel
  (bind _returnvalue (Game|GetPlayerController 0))
  (bind _hitresult (Game|Player|GetHitResultUnderCursorbyChannel _returnvalue "TraceTypeQuery1" false))
  (bind (_bblockinghit _binitialoverlap _time _distance _location _impactpoint _normal _impactnormal _physmat _hitactor) (Collision|BreakHitResult _hitresult))
  (Utilities|IsValid _hitactor
    (:Is%20Valid
      (bind _asbp_trcg_display_card (Utilities|Casting|CastToBP_TRCG_DisplayCard _hitactor))
      (Variables|/Game/TRCG/Gameplay/Cards/Display/BP_TRCG_DisplayCard.BP_TRCG_DisplayCard_C|SetFocusAngle _asbp_trcg_display_card _impactpoint))))