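; Manager for planet stats (pressure, temperature, breathability) and their target objectives, registered on the game instance as StatManager.
; On BeginPlay it constructs one object per stat class for both the current Stats and the Objectives collections, with different starting values.
; Helper functions find a stat by class in a given collection and add to a stat's value within a clamped range.
; A bound log event prints both collections for debugging.
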(event Custom|OnLogManagedCalled
  (Development|PrintString "===================" false)
  (Development|PrintString "STATS" false)
  (for _array_element (Variables|Default|GetStats)
    (Development|PrintString (Utilities|String|ToString(Text) (Variables|/Script/TerraCardGame.TrcgPlanetStat|GetName _array_element)) false)
    (Development|PrintString (Utilities|String|ToString(Integer) (Variables|/Script/TerraCardGame.TrcgPlanetStat|GetValue _array_element)) false))
  (Development|PrintString "----------------------" false)
  (Development|PrintString "OBJECTIVES" false)
  (for _array_element_2 (Variables|Default|GetObjectives)
    (Development|PrintString (Utilities|String|ToString(Text) (Variables|/Script/TerraCardGame.TrcgPlanetStat|GetName _array_element_2)) false)
    (Development|PrintString (Utilities|String|ToString(Integer) (Variables|/Script/TerraCardGame.TrcgPlanetStat|GetValue _array_element_2)) false)
    (Development|PrintString "===================" false)))

(event EventBeginPlay
  (EventDispatchers|BindEventtoLogManagedStats (delegate Custom|OnLogManagedCalled))
  (Variables|/Script/TerraCardGame.TrcgGameInstance|SetStatManager (Class|TrcgActor|GetTrcgGameInstance) self)
  (bind _returnvalue (Game|ConstructObjectfromClass "/Game/TRCG/Gameplay/Stats/BP_TRCG_PlanetStat_Pressure.BP_TRCG_PlanetStat_Pressure_C"))
  (Utilities|Array|Add (Variables|Default|GetStats) _returnvalue)
  (bind _returnvalue_2 (Game|ConstructObjectfromClass "/Game/TRCG/Gameplay/Stats/BP_TRCG_PlanetStat_Temperature.BP_TRCG_PlanetStat_Temperature_C"))
  (Utilities|Array|Add (Variables|Default|GetStats) _returnvalue_2)
  (bind _returnvalue_3 (Game|ConstructObjectfromClass "/Game/TRCG/Gameplay/Stats/BP_TRCG_PlanetStat_Breathability.BP_TRCG_PlanetStat_Breathability_C"))
  (Utilities|Array|Add (Variables|Default|GetStats) _returnvalue_3)
  (bind _returnvalue_4 (Game|ConstructObjectfromClass "/Game/TRCG/Gameplay/Stats/BP_TRCG_PlanetStat_Pressure.BP_TRCG_PlanetStat_Pressure_C" 10))
  (Utilities|Array|Add (Variables|Default|GetObjectives) _returnvalue_4)
  (bind _returnvalue_5 (Game|ConstructObjectfromClass "/Game/TRCG/Gameplay/Stats/BP_TRCG_PlanetStat_Temperature.BP_TRCG_PlanetStat_Temperature_C" 10))
  (Utilities|Array|Add (Variables|Default|GetObjectives) _returnvalue_5)
  (bind _returnvalue_6 (Game|ConstructObjectfromClass "/Game/TRCG/Gameplay/Stats/BP_TRCG_PlanetStat_Breathability.BP_TRCG_PlanetStat_Breathability_C" 10))
  (Utilities|Array|Add (Variables|Default|GetObjectives) _returnvalue_6))

(fn ConstructionScript)

(fn ApplyChangetoStat
  (params (Stat :type Trcg%20Planet%20Stat%20Object%20Reference) (ValueToAdd :type Integer))
  (Variables|/Script/TerraCardGame.TrcgPlanetStat|SetValue Stat (Math|Integer|Clamp(Integer) (+ (Variables|/Script/TerraCardGame.TrcgPlanetStat|GetValue Stat) ValueToAdd) 0 20))
  (return))

(fn GetStatbyClass
  (params (StatClass :type BP%20TRCG%20Planet%20Stat%20Class%20Reference) (FromCollection :type Array%20of%20Trcg%20Planet%20Stat%20Object%20References))
  (for _array_element FromCollection
    (if (== StatClass (Utilities|GetClass _array_element))
      (return _array_element)))
  (return 0))