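; BP_TRCG_Hand is the base Blueprint for a hand of cards in the TRCG card game.
; It keeps the cards in an array, with functions to add a card and to clear the whole hand.
; IsFull compares the card count against MaxSize, but AddCard itself does not enforce that limit.
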(fn AddCard
  (params (Card :type BP%20TRCG%20Card%20Object%20Reference))
  (Utilities|Array|Add (Variables|Default|GetCards) Card)
  (return))

(fn Empty
  (Utilities|Array|Clear (Variables|Default|GetCards))
  (return))

(fn IsFull
  (return (>= (Utilities|Array|Length (Variables|Default|GetCards)) (Variables|Default|GetMaxSize))))