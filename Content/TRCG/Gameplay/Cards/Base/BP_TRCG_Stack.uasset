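; BP_TRCG_Stack is a base card stack for the TRCG card game, holding cards in a Cards array.
; It exposes functions to add a card, returning the array's Add result, shuffle the stack in place, and empty it.
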(fn AddCard
  (params (Card :type BP%20TRCG%20Card%20Object%20Reference))
  (bind _returnvalue (Utilities|Array|Add (Variables|Default|GetCards) Card))
  (return _returnvalue))

(fn Shuffle
  (Utilities|Array|Shuffle (Variables|Default|GetCards))
  (return))

(fn Empty
  (Utilities|Array|Clear (Variables|Default|GetCards))
  (return))