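; Card manager that owns the deck, action, construction and discard stacks, and the hand.
; On BeginPlay it creates these containers, then replaces the deck with debug cards, sorts them by type into shuffled stacks and opens a debug widget.
; Picks move action cards from the stack's end and construction cards from its front into the hand.
; Playing uses a card on a random tile index, then discards it; changes trigger logging.
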(event Custom|Debug
  (bind _returnvalue (Game|ConstructObjectfromClass "/Game/TRCG/Gameplay/Cards/Base/BP_TRCG_Card_Action.BP_TRCG_Card_Action_C" "/Game/TRCG/Gameplay/Cards/Data/Debug/DA_TRCG_CD_DebugAction.DA_TRCG_CD_DebugAction"))
  (bind _returnvalue_2 (Game|ConstructObjectfromClass "/Game/TRCG/Gameplay/Cards/Base/BP_TRCG_Card_Action.BP_TRCG_Card_Action_C" "/Game/TRCG/Gameplay/Cards/Data/Debug/DA_TRCG_CD_DebugActionBis.DA_TRCG_CD_DebugActionBis"))
  (bind _returnvalue_3 (Game|ConstructObjectfromClass "/Game/TRCG/Gameplay/Cards/Base/BP_TRCG_Card_Construction.BP_TRCG_Card_Construction_C" "/Game/TRCG/Gameplay/Cards/Data/Debug/DA_TRCG_CD_DebugConstructionBis.DA_TRCG_CD_DebugConstructionBis"))
  (bind _returnvalue_4 (Game|ConstructObjectfromClass "/Game/TRCG/Gameplay/Cards/Base/BP_TRCG_Card_Construction.BP_TRCG_Card_Construction_C" "/Game/TRCG/Gameplay/Cards/Data/Debug/DA_TRCG_CD_DebugConstruction.DA_TRCG_CD_DebugConstruction"))
  (bind _returnvalue_5 (Game|ConstructObjectfromClass "/Game/TRCG/Gameplay/Cards/Base/BP_TRCG_Deck.BP_TRCG_Deck_C" (Utilities|Array|MakeArray _returnvalue _returnvalue_2 _returnvalue_3 _returnvalue_4)))
  (Variables|Default|SetDeck _returnvalue_5)
  (CallFunction|FillStacksfromDeck)
  (bind _returnvalue_6 (UserInterface|CreateWidget "/Game/TRCG/HUD/WBP_Debug.WBP_Debug_C" (Game|GetPlayerController 0) self))
  (UserInterface|Viewport|AddtoViewport _returnvalue_6 0))

(event Custom|OnLogManagedCalled
  (bind _returnvalue (Class|TrcgActor|GetTrcgGameInstance))
  (bind _statmanager (Variables|/Script/TerraCardGame.TrcgGameInstance|GetStatManager _returnvalue))
  (Development|PrintString "===================" false)
  (Development|PrintString "DECK :" false)
  (for _array_element (Variables|/Game/TRCG/Gameplay/Cards/Base/BP_TRCG_Deck.BP_TRCG_Deck_C|GetCards (Variables|Default|GetDeck))
    (Development|PrintString (Utilities|String|ToString(Text) (Variables|/Script/TerraCardGame.TrcgCardData|GetCardName (Variables|/Game/TRCG/Gameplay/Cards/Base/BP_TRCG_Card.BP_TRCG_Card_C|GetData _array_element))) false))
  (Development|PrintString "ACTION STACK :" false)
  (for _array_element_2 (Variables|/Game/TRCG/Gameplay/Cards/Base/BP_TRCG_Stack.BP_TRCG_Stack_C|GetCards (Variables|Default|GetActionStack))
    (Development|PrintString (Utilities|String|ToString(Text) (Variables|/Script/TerraCardGame.TrcgCardData|GetCardName (Variables|/Game/TRCG/Gameplay/Cards/Base/BP_TRCG_Card.BP_TRCG_Card_C|GetData _array_element_2))) false))
  (Development|PrintString "CONSTRUCTION STACK :" false)
  (for _array_element_3 (Variables|/Game/TRCG/Gameplay/Cards/Base/BP_TRCG_Stack.BP_TRCG_Stack_C|GetCards (Variables|Default|GetConstructionStack))
    (Development|PrintString (Utilities|String|ToString(Text) (Variables|/Script/TerraCardGame.TrcgCardData|GetCardName (Variables|/Game/TRCG/Gameplay/Cards/Base/BP_TRCG_Card.BP_TRCG_Card_C|GetData _array_element_3))) false))
  (Development|PrintString "DISCARD STACK :" false)
  (for _array_element_4 (Variables|/Game/TRCG/Gameplay/Cards/Base/BP_TRCG_Stack.BP_TRCG_Stack_C|GetCards (Variables|Default|GetDiscardStack))
    (Development|PrintString (Utilities|String|ToString(Text) (Variables|/Script/TerraCardGame.TrcgCardData|GetCardName (Variables|/Game/TRCG/Gameplay/Cards/Base/BP_TRCG_Card.BP_TRCG_Card_C|GetData _array_element_4))) false))
  (Development|PrintString "HAND :" false)
  (for _array_element_5 (Variables|/Game/TRCG/Gameplay/Cards/Base/BP_TRCG_Hand.BP_TRCG_Hand_C|GetCards (Variables|Default|GetHand))
    (Development|PrintString (Utilities|String|ToString(Text) (Variables|/Script/TerraCardGame.TrcgCardData|GetCardName (Variables|/Game/TRCG/Gameplay/Cards/Base/BP_TRCG_Card.BP_TRCG_Card_C|GetData _array_element_5))) false))
  (Development|PrintString "===================" false)
  (Utilities|IsValid _statmanager
    (:Is%20Valid
      (bind _asbp_trcg_planet_stats_manager (Utilities|Casting|CastToBP_TRCG_PlanetStatsManager _statmanager))
      (Default|CallLogManagedStats _asbp_trcg_planet_stats_manager))))

(event EventBeginPlay
  (EventDispatchers|BindEventtoLogManagedCards (delegate Custom|OnLogManagedCalled))
  (bind _returnvalue (Game|ConstructObjectfromClass "/Game/TRCG/Gameplay/Cards/Base/BP_TRCG_Deck.BP_TRCG_Deck_C"))
  (Variables|Default|SetDeck _returnvalue)
  (bind _returnvalue_2 (Game|ConstructObjectfromClass "/Game/TRCG/Gameplay/Cards/Base/BP_TRCG_Stack_Action.BP_TRCG_Stack_Action_C"))
  (Variables|Default|SetActionStack _returnvalue_2)
  (bind _returnvalue_3 (Game|ConstructObjectfromClass "/Game/TRCG/Gameplay/Cards/Base/BP_TRCG_Stack_Construction.BP_TRCG_Stack_Construction_C"))
  (Variables|Default|SetConstructionStack _returnvalue_3)
  (bind _returnvalue_4 (Game|ConstructObjectfromClass "/Game/TRCG/Gameplay/Cards/Base/BP_TRCG_Stack_Discard.BP_TRCG_Stack_Discard_C"))
  (Variables|Default|SetDiscardStack _returnvalue_4)
  (bind _returnvalue_5 (Game|ConstructObjectfromClass "/Game/TRCG/Gameplay/Cards/Base/BP_TRCG_Hand.BP_TRCG_Hand_C"))
  (Variables|Default|SetHand _returnvalue_5)
  (if (Math|Boolean|ANDBoolean (Utilities|IsValid (Variables|Default|GetDeck)) (Utilities|IsValid (Variables|Default|GetActionStack)) (Utilities|IsValid (Variables|Default|GetConstructionStack)) (Utilities|IsValid (Variables|Default|GetDiscardStack)) (Utilities|IsValid (Variables|Default|GetHand)))
    (CallFunction|Debug)
    (else
      (Development|PrintString "ERROR ON INIT" true true "(R=1.000000,G=0.000000,B=0.000000,A=1.000000)"))))

(fn ConstructionScript)

(fn FillStacksfromDeck
  (for _array_element (Variables|/Game/TRCG/Gameplay/Cards/Base/BP_TRCG_Deck.BP_TRCG_Deck_C|GetCards (Variables|Default|GetDeck))
    (bind _asbp_trcg_card_action (Utilities|Casting|CastToBP_TRCG_Card_Action _array_element)
      (:then
        (Default|AddCard (Variables|Default|GetActionStack) _asbp_trcg_card_action))
      (:CastFailed
        (bind _asbp_trcg_card_construction (Utilities|Casting|CastToBP_TRCG_Card_Construction _array_element)
          (:then
            (Default|AddCard (Variables|Default|GetConstructionStack) _asbp_trcg_card_construction))
          (:CastFailed
            (Development|PrintString "ERROR ON FILLCARDSFROMDECK" true true "(R=1.000000,G=0.000000,B=0.000000,A=1.000000)"))))))
  (CallFunction|ShuffleAllStacks)
  (Default|CallLogManagedCards)
  (return))

(fn PickActionCard
  (bind _actionstack (Variables|Default|GetActionStack))
  (bind _cards (Variables|/Game/TRCG/Gameplay/Cards/Base/BP_TRCG_Stack.BP_TRCG_Stack_C|GetCards _actionstack))
  (bind _returnvalue (Utilities|Array|LastIndex _cards))
  (bind _output (Utilities|Array|Get(acopy) _cards _returnvalue))
  (Default|AddCard (Variables|Default|GetHand) _output)
  (Utilities|Array|RemoveItem _cards _output)
  (Default|CallLogManagedCards)
  (return))

(fn ShuffleAllStacks
  (Default|Shuffle (Variables|Default|GetActionStack))
  (Default|Shuffle (Variables|Default|GetConstructionStack))
  (return))

(fn PickConstructionCard
  (bind _constructionstack (Variables|Default|GetConstructionStack))
  (bind _cards (Variables|/Game/TRCG/Gameplay/Cards/Base/BP_TRCG_Stack.BP_TRCG_Stack_C|GetCards _constructionstack))
  (bind _output (Utilities|Array|Get(acopy) _cards))
  (Default|AddCard (Variables|Default|GetHand) _output)
  (Utilities|Array|RemoveItem _cards _output)
  (Default|CallLogManagedCards)
  (return))

(fn PlayCardfromHand
  (params (CardIndex :type Integer))
  (bind _hand (Variables|Default|GetHand))
  (bind _cards (Variables|/Game/TRCG/Gameplay/Cards/Base/BP_TRCG_Hand.BP_TRCG_Hand_C|GetCards _hand))
  (bind _output (Utilities|Array|Get(acopy) _cards CardIndex))
  (Default|UseCard _output (Math|Random|RandomIntegerinRange 0 (- (Utilities|Array|Length (Variables|/Script/TerraCardGame.TrcgTileManager|GetTiles (Variables|/Script/TerraCardGame.TrcgGameInstance|GetTileManager (Class|TrcgActor|GetTrcgGameInstance)))) 1)))
  (Default|AddCard (Variables|Default|GetDiscardStack) _output)
  (Utilities|Array|RemoveItem _cards _output)
  (Default|CallLogManagedCards)
  (return))