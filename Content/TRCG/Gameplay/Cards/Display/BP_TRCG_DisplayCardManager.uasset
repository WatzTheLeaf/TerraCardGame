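; Card gallery manager that lays out every card from the TRCG game instance's CardData as a browsable grid.
; On BeginPlay, BuildGrid spawns a display card per entry, deriving row and column from its index, column count, card size and padding.
; It then teleports the player pawn to the computed grid center, keeping its height, and spawns a blocking volume there, sized from the grid extents plus a margin.
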(event EventBeginPlay
  (CallFunction|BuildGrid))

(fn ConstructionScript)

(fn BuildGrid
  (bind _returnvalue (Game|Player|GetPlayerPawn 0))
  (bind _returnvalue_2 (Class|TrcgActor|GetTrcgGameInstance))
  (bind _numcol (Variables|Default|GetNumCol))
  (bind _cardpadding (Variables|Default|GetCardPadding))
  (bind _cardsize (Variables|Default|GetCardSize))
  (bind _cardsize_2 (Variables|Default|GetCardSize))
  (bind _cardpadding_2 (Variables|Default|GetCardPadding))
  (bind _cardsize_3 (Variables|Default|GetCardSize))
  (bind _cardsize_4 (Variables|Default|GetCardSize))
  (bind _cardpadding_3 (Variables|Default|GetCardPadding))
  (bind _numcol_2 (Variables|Default|GetNumCol))
  (bind _cardpadding_4 (Variables|Default|GetCardPadding))
  (bind _returnvalue_3 (+ _cardsize_2 _cardpadding_3))
  (bind _returnvalue_4 (+ _cardpadding _cardsize_4))
  (bind _returnvalue_5 (+ _cardpadding_4 _cardsize))
  (bind _carddata (Variables|/Script/TerraCardGame.TrcgGameInstance|GetCardData _returnvalue_2))
  (bind _returnvalue_6 (Utilities|Array|Length _carddata))
  (bind _returnvalue_7 (* _numcol _returnvalue_4))
  (bind _returnvalue_8 (Utilities|Operators|Subtract _returnvalue_7 _cardsize_3 _cardpadding_2))
  (bind _returnvalue_9 (- _returnvalue_6 1))
  (bind _returnvalue_10 (/ _returnvalue_9 _numcol_2))
  (bind _returnvalue_11 (/ _returnvalue_8 2.0))
  (bind _returnvalue_12 (* _returnvalue_10 _returnvalue_5))
  (bind _returnvalue_13 (/ _returnvalue_12 2.0))
  (Utilities|FlowControl|Sequence
    (:then_0
      (for (_array_element _array_index) (Variables|/Script/TerraCardGame.TrcgGameInstance|GetCardData (Class|TrcgActor|GetTrcgGameInstance))
        (Game|SpawnActorfromClass "/Game/TRCG/Gameplay/Cards/Display/BP_TRCG_DisplayCard.BP_TRCG_DisplayCard_C" (Math|Transform|MakeTransform (+ (Variables|Default|GetSpawnOrigin) (Math|Vector|MakeVector (* _returnvalue_3 (/ _array_index (Variables|Default|GetNumCol))) (* _returnvalue_3 (Math|Integer|%(Integer) _array_index (Variables|Default|GetNumCol))) 0.0)) "0.000000,90.000000,0.000000") "Undefined" "MultiplyWithRoot" 0 _array_element 0)))
    (:then_1
      (Transformation|Teleport _returnvalue (Math|Vector|MakeVector _returnvalue_13 _returnvalue_11 (.z (Transformation|GetActorLocation _returnvalue))) (Transformation|GetActorRotation _returnvalue))
      (Game|SpawnActorfromClass "/Game/TRCG/Gameplay/Misc/BP_TRCG_BlockingVolume.BP_TRCG_BlockingVolume_C" (Math|Transform|MakeTransform (Math|Vector|MakeVector _returnvalue_13 _returnvalue_11 (.z (Variables|Default|GetSpawnOrigin)))) "Undefined" "MultiplyWithRoot" 0 (Math|Vector2D|MakeVector2D (+ _returnvalue_11 3e+02) (+ _returnvalue_13 3e+02)) 0))))