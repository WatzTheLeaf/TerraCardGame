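; Display card actor that shows a card's material, name and description and tilts with a hover effect.
; On BeginPlay it applies the card data to the mesh and to a WBP_CardText widget.
; Each tick, LerpHoverRotation maps the FocusAngle point's offset from the card to clamped pitch and roll, interpolating rotation at a fixed yaw.
; FocusAngle continually eases back to the actor's location, so the tilt settles to neutral.
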(event EventTick
  (params (DeltaSeconds :type Float%20%28single-precision%29))
  (CallFunction|LerpHoverRotation (Variables|Default|GetFocusAngle) DeltaSeconds)
  (Variables|Default|SetFocusAngle (Math|Interpolation|VInterpTo (Variables|Default|GetFocusAngle) (Transformation|GetActorLocation) DeltaSeconds 2.0)))

(event EventBeginPlay
  (bind _data (Variables|Default|GetData))
  (Rendering|Material|SetMaterial (Variables|Default|GetCardMesh) 0 (Variables|/Script/TerraCardGame.TrcgCardData|GetMaterial (Variables|Default|GetData)))
  (bind _aswbp_card_text (Utilities|Casting|CastToWBP_CardText (UserInterface|GetWidget (Variables|Default|GetWidget))))
  (Variables|/Game/TRCG/HUD/WBP_CardText.WBP_CardText_C|SetCardTitle _aswbp_card_text (Variables|/Script/TerraCardGame.TrcgCardData|GetCardName _data))
  (Variables|/Game/TRCG/HUD/WBP_CardText.WBP_CardText_C|SetCardDesc _aswbp_card_text (Variables|/Script/TerraCardGame.TrcgCardData|GetCardDesc _data)))

(fn ConstructionScript)

(fn LerpHoverRotation
  (params (ImpactPoint :type Vector) (Delta :type Float%20%28double-precision%29))
  (bind _returnvalue (Transformation|GetActorLocation))
  (bind _tiltangle (Variables|Default|GetTiltAngle))
  (bind _tiltangle_2 (Variables|Default|GetTiltAngle))
  (bind _anchor (Variables|Default|GetAnchor))
  (bind _returnvalue_2 (Transformation|GetRelativeTransform _anchor))
  (bind _returnvalue_3 (- ImpactPoint _returnvalue))
  (bind _returnvalue_4 (Math|Transform|InverseTransformLocation _returnvalue_2 _returnvalue_3))
  (LocalVariables|SetPitch (Math|Float|MapRangeClamped (.y _returnvalue_4) -5e+01 5e+01 _tiltangle_2 (- 0.0 _tiltangle_2)))
  (LocalVariables|SetRoll (Math|Float|MapRangeClamped (.x _returnvalue_4) -5e+01 5e+01 _tiltangle (- 0.0 _tiltangle)))
  (Transformation|SetActorRotation (Math|Interpolation|RInterpTo (Transformation|GetActorRotation) (Math|Rotator|MakeRotator (LocalVariables|GetRoll) (LocalVariables|GetPitch) 9e+01) Delta 5.0)))