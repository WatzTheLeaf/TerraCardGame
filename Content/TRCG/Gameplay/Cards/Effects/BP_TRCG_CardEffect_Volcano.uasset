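; Card effect Blueprint for the Volcano card, which turns the targeted tile into a volcano and affects the tiles around it.
; StartEffect applies the Volcano biome interaction to the target tile, then checks each neighbour from the TileManager by gameplay tag.
; Forest and Ocean neighbours receive their own volcano interaction data assets.
; Each affected tile also has its mesh material swapped to a coloured debug material.
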(event EventStartEffect
  (params (OnTile :type Integer))
  (bind _returnvalue (Class|TrcgObject|GetTrcgGameInstance))
  (bind _tilemanager (Variables|/Script/TerraCardGame.TrcgGameInstance|GetTileManager _returnvalue))
  (Class|TrcgCardEffect|ApplyBiomeInteraction "/Game/TRCG/Data/Biomes/DA_TRCG_BI_Volcano.DA_TRCG_BI_Volcano" OnTile)
  (Rendering|Material|SetMaterial (Variables|/Script/TerraCardGame.TrcgTile|GetMesh (Class|TrcgTileManager|GetTileatIndex _tilemanager OnTile)) 0 "/Game/TRCG/Assets/Materials/World/Debug/M_DebugTile_Red.M_DebugTile_Red")
  (bind _returnvalue_2 (Class|TrcgTileManager|GetNeighbourTiles _tilemanager OnTile))
  (for _array_element _returnvalue_2
    (if (GameplayTags|HasTag (Variables|/Script/TerraCardGame.TrcgTile|GetTileTags _array_element) "(TagName=\"Tiles.Type.Forest\")" true)
      (Class|TrcgCardEffect|ApplyBiomeInteractionwithRef "/Game/TRCG/Data/Biomes/DA_TRCG_BI_Forest_Volcano.DA_TRCG_BI_Forest_Volcano" _array_element)
      (Rendering|Material|SetMaterial (Variables|/Script/TerraCardGame.TrcgTile|GetMesh _array_element) 0 "/Game/TRCG/Assets/Materials/World/Debug/M_DebugTile_LightGray.M_DebugTile_LightGray")
      (elif (GameplayTags|HasTag (Variables|/Script/TerraCardGame.TrcgTile|GetTileTags _array_element) "(TagName=\"Tiles.Type.Ocean\")" true)
        (Class|TrcgCardEffect|ApplyBiomeInteractionwithRef "/Game/TRCG/Data/Biomes/DA_TRCG_BI_Ocean_Volcano.DA_TRCG_BI_Ocean_Volcano" _array_element)
        (Rendering|Material|SetMaterial (Variables|/Script/TerraCardGame.TrcgTile|GetMesh _array_element) 0 "/Game/TRCG/Assets/Materials/World/Debug/M_DebugTile_Black.M_DebugTile_Black")))))