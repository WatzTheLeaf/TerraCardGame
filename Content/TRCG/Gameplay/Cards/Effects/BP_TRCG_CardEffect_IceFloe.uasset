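; Card effect for the Ice Floe card, applying a biome interaction to the target tile.
; If a neighbouring tile has the Volcano tag, it uses the Ocean-Volcano interaction data and a black debug material instead of the Ice Floe data and ice debug material.
; PreviewEffect repeats the same neighbour check and returns the matching stat changes without altering the tile.
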(event EventStartEffect
  (params (OnTile :type Integer))
  (bind _returnvalue (Class|TrcgObject|GetTrcgGameInstance))
  (bind _tilemanager (Variables|/Script/TerraCardGame.TrcgGameInstance|GetTileManager _returnvalue))
  (bind _returnvalue_2 (Class|TrcgTileManager|GetTileatIndex _tilemanager OnTile))
  (bind _mesh (Variables|/Script/TerraCardGame.TrcgTile|GetMesh _returnvalue_2))
  (if (Class|TrcgTileManager|HasNeighbourTileswithTileTag _tilemanager OnTile "(TagName=\"Tiles.Type.Volcano\")")
    (Class|TrcgCardEffect|ApplyBiomeInteraction "/Game/TRCG/Data/Biomes/DA_TRCG_BI_Ocean_Volcano.DA_TRCG_BI_Ocean_Volcano" OnTile)
    (Rendering|Material|SetMaterial _mesh 0 "/Game/TRCG/Assets/Materials/World/Debug/M_DebugTile_Black.M_DebugTile_Black")
    (else
      (Class|TrcgCardEffect|ApplyBiomeInteraction "/Game/TRCG/Data/Biomes/DA_TRCG_BI_IceFloe.DA_TRCG_BI_IceFloe" OnTile)
      (Rendering|Material|SetMaterial _mesh 0 "/Game/TRCG/Assets/Materials/World/Debug/M_DebugTile_Ice.M_DebugTile_Ice"))))

(fn PreviewEffect
  (params (OnTile :type Integer))
  (if (Class|TrcgTileManager|HasNeighbourTileswithTileTag (Variables|/Script/TerraCardGame.TrcgGameInstance|GetTileManager (Class|TrcgObject|GetTrcgGameInstance)) OnTile "(TagName=\"Tiles.Type.Volcano\")")
    (bind _returnvalue (Class|TrcgCardEffect|StatChangesfromData "/Game/TRCG/Data/Biomes/DA_TRCG_BI_Ocean_Volcano.DA_TRCG_BI_Ocean_Volcano"))
    (return _returnvalue)
    (else
      (bind _returnvalue_2 (Class|TrcgCardEffect|StatChangesfromData "/Game/TRCG/Data/Biomes/DA_TRCG_BI_IceFloe.DA_TRCG_BI_IceFloe"))
      (return _returnvalue_2))))