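; Card effect Blueprint for the Ocean card, which changes the tile it is played on and the planet's stats.
; StartEffect asks the game instance's TileManager whether a neighbouring tile is tagged Volcano.
; Next to a volcano the tile becomes LavaRocks with a black debug material and raises Pressure.
; Otherwise it becomes Ocean with a blue debug material, lowering Temperature and raising Pressure through the StatManager.
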(event EventStartEffect
  (params (OnTile :type Integer))
  (bind _returnvalue (Class|TrcgObject|GetTrcgGameInstance))
  (bind _statmanager (Variables|/Script/TerraCardGame.TrcgGameInstance|GetStatManager _returnvalue))
  (bind _tilemanager (Variables|/Script/TerraCardGame.TrcgGameInstance|GetTileManager _returnvalue))
  (bind _returnvalue_2 (Class|TrcgTileManager|GetTileatIndex _tilemanager OnTile))
  (bind _returnvalue_3 (Class|TrcgPlanetStatsManager|GetStatfromClass _statmanager "/Game/TRCG/Gameplay/Stats/BP_TRCG_PlanetStat_Pressure.BP_TRCG_PlanetStat_Pressure_C"))
  (bind _mesh (Variables|/Script/TerraCardGame.TrcgTile|GetMesh _returnvalue_2))
  (if (Class|TrcgTileManager|HasNeighbourTileswithTileTag _tilemanager OnTile "(TagName=\"Tiles.Type.Volcano\")")
    (Variables|/Script/TerraCardGame.TrcgTile|SetTileTags _returnvalue_2 "(GameplayTags=((TagName=\"Tiles.Type.LavaRocks\")))")
    (Rendering|Material|SetMaterial _mesh 0 "/Game/TRCG/Assets/Materials/World/Debug/M_DebugTile_Black.M_DebugTile_Black")
    (Class|TrcgPlanetStat|ApplyStatChange _returnvalue_3 1)
    (else
      (Variables|/Script/TerraCardGame.TrcgTile|SetTileTags _returnvalue_2 "(GameplayTags=((TagName=\"Tiles.Type.Ocean\")))")
      (Rendering|Material|SetMaterial _mesh 0 "/Game/TRCG/Assets/Materials/World/Debug/M_DebugTile_Blue.M_DebugTile_Blue")
      (Class|TrcgPlanetStat|ApplyStatChange (Class|TrcgPlanetStatsManager|GetStatfromClass _statmanager "/Game/TRCG/Gameplay/Stats/BP_TRCG_PlanetStat_Temperature.BP_TRCG_PlanetStat_Temperature_C") -1)
      (Class|TrcgPlanetStat|ApplyStatChange _returnvalue_3 1))))