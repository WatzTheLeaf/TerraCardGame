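; Debug card effect for TRCG that visualizes a target tile and its neighbours by recolouring their meshes.
; On StartEffect, it looks up the tile at the given index through the game instance's TileManager and applies a red debug material to it.
; It then gets that tile's neighbours from the same manager and applies a green debug material to each valid one.
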(event EventStartEffect
  (params (OnTile :type Integer))
  ;[1 1 1] Testing
  (Rendering|Material|SetMaterial (Variables|/Script/TerraCardGame.TrcgTile|GetMesh (Class|TrcgTileManager|GetTileatIndex (Variables|/Script/TerraCardGame.TrcgGameInstance|GetTileManager (Class|TrcgObject|GetTrcgGameInstance)) OnTile)) 0 "/Game/TRCG/Assets/Materials/M_DebugTile_Red.M_DebugTile_Red")
  (bind _returnvalue (Class|TrcgTileManager|GetNeighbourTiles (Variables|/Script/TerraCardGame.TrcgGameInstance|GetTileManager (Class|TrcgObject|GetTrcgGameInstance)) OnTile))
  (for _array_element _returnvalue
    (Utilities|IsValid _array_element
      (:Is%20Valid
        (Rendering|Material|SetMaterial (Variables|/Script/TerraCardGame.TrcgTile|GetMesh _array_element) 0 "/Game/TRCG/Assets/Materials/M_DebugTile_Green.M_DebugTile_Green")))))