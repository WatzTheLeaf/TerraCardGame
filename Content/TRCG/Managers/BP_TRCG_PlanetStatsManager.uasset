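; BP_TRCG_PlanetStatsManager holds the current planet's stats and their target objectives, registering itself on the game instance at BeginPlay.
; It builds both collections from the level data's StatConditions map, creating an object per stat class with X as starting value and Y as objective.
; Helpers find a stat by class and apply changes clamped to the level's Range.
; A bound log event prints both collections for debugging.
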(event Custom|OnLogManagedCalled
  (Development|PrintString "===================" false)
  (Development|PrintString "STATS" false)
  (for _array_element (Variables|Default|GetStats)
    (Development|PrintString (Utilities|String|ToString(Text) (Variables|/Script/TerraCardGame.TrcgPlanetStat|GetName _array_element)) false)
    (Development|PrintString (Utilities|String|ToString(Integer) (Variables|/Script/TerraCardGame.TrcgPlanetStat|GetValue _array_element)) false))
  (Development|PrintString "----------------------" false)
  (Development|PrintString "OBJECTIVES" false)
  (for _array_element_2 (Variables|Default|GetObjectives)
    (Development|PrintString (Utilities|String|ToString(Text) (Variables|/Script/TerraCardGame.TrcgPlanetStat|GetName _array_element_2)) false)
    (Development|PrintString (Utilities|String|ToString(Integer) (Variables|/Script/TerraCardGame.TrcgPlanetStat|GetValue _array_element_2)) false)
    (Development|PrintString "===================" false)))

(event EventBeginPlay
  (bind _returnvalue (Class|TrcgActor|GetTrcgGameInstance))
  (EventDispatchers|BindEventtoLogManagedStats (delegate Custom|OnLogManagedCalled))
  (Variables|/Script/TerraCardGame.TrcgGameInstance|SetStatManager _returnvalue self)
  (CallFunction|InitPlanetfromData (Variables|/Script/TerraCardGame.TrcgGameInstance|GetCurrentLevelData _returnvalue)))

(fn ConstructionScript)

(fn ApplyChangetoStat
  (params (Stat :type Trcg%20Planet%20Stat%20Object%20Reference) (ValueToAdd :type Integer))
  (bind _returnvalue (Class|TrcgActor|GetTrcgGameInstance))
  (bind _currentleveldata (Variables|/Script/TerraCardGame.TrcgGameInstance|GetCurrentLevelData _returnvalue))
  (bind _range (Variables|/Script/TerraCardGame.TrcgLevelPlanetData|GetRange _currentleveldata))
  (Variables|/Script/TerraCardGame.TrcgPlanetStat|SetValue Stat (Math|Integer|Clamp(Integer) (+ (Variables|/Script/TerraCardGame.TrcgPlanetStat|GetValue Stat) ValueToAdd) (.x _range) (.y _range)))
  (return))

(fn GetStatbyClass
  (params (StatClass :type BP%20TRCG%20Planet%20Stat%20Class%20Reference) (FromCollection :type Array%20of%20Trcg%20Planet%20Stat%20Object%20References))
  (for _array_element FromCollection
    (if (== StatClass (Utilities|GetClass _array_element))
      (return _array_element)))
  (return 0))

(fn InitPlanetfromData
  (params (Data :type Trcg%20Level%20Planet%20Data%20Object%20Reference))
  (bind _statconditions (Variables|/Script/TerraCardGame.TrcgLevelPlanetData|GetStatConditions Data))
  (Utilities|IsValid Data
    (:Is%20Valid
      (bind _keys (Utilities|Map|Keys _statconditions))
      (for _array_element _keys
        (bind _returnvalue (Game|ConstructObjectfromClass _array_element (.x (.Value (Utilities|Map|Find _statconditions _array_element)))))
        (Utilities|Array|Add (Variables|Default|GetStats) _returnvalue))
      (bind _keys_2 (Utilities|Map|Keys _statconditions))
      (for _array_element_2 _keys_2
        (bind _returnvalue_2 (Game|ConstructObjectfromClass _array_element_2 (.y (.Value (Utilities|Map|Find _statconditions _array_element_2)))))
        (Utilities|Array|Add (Variables|Default|GetObjectives) _returnvalue_2)))))