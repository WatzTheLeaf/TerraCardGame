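; Card manager for the TRCG card game, owning the deck, Action, Construction, Discard and Recycle stacks, and the hand.
; It builds the deck from the game instance's GlobalDeck, registers itself there, then splits cards by type into shuffled stacks.
; Played cards need tags matching the tile and move to Discard; reshuffles rebuild stacks from the master deck.
; Recycling removes cards from that deck, and a new card can replace them.
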(event Custom|OnLogManagedCalled
  (bind _returnvalue (Class|TrcgActor|GetTrcgGameInstance))
  (bind _statmanager (Variables|/Script/TerraCardGame.TrcgGameInstance|GetStatManager _returnvalue))
  (Development|PrintString "===================" false)
  (Development|PrintString "DECK :" false)
  (for _array_element (Variables|/Game/TRCG/Gameplay/Cards/Base/BP_TRCG_Deck.BP_TRCG_Deck_C|GetCards (Variables|Default|GetDeck))
    (Development|PrintString (Utilities|String|ToString(Text) (Variables|/Script/TerraCardGame.TrcgCardData|GetCardName (Variables|/Game/TRCG/Gameplay/Cards/Base/BP_TRCG_Card.BP_TRCG_Card_C|GetData _array_element))) false))
  (Development|PrintString "ACTION STACK :" false)
  (for _array_element_2 (Variables|/Game/TRCG/Gameplay/Cards/Base/BP_TRCG_Stack.BP_TRCG_Stack_C|GetCards (Variables|Default|GetActionStack))
    (Development|PrintString (Utilities|String|ToString(Text) (Variables|/Script/TerraCardGame.TrcgCardData|GetCardName (Variables|/Game/TRCG/Gameplay/Cards/Base/BP_TRCG_Card.BP_TRCG_Card_C|GetData _array_element_2))) false))
  (Development|PrintString "CONSTRUCTION STACK :" false)
  (for _array_element_3 (Variables|/Game/TRCG/Gameplay/Cards/Base/BP_TRCG_Stack.BP_TRCG_Stack_C|GetCards (Variables|Default|GetConstructionStack))
    (Development|PrintString (Utilities|String|ToString(Text) (Variables|/Script/TerraCardGame.TrcgCardData|GetCardName (Variables|/Game/TRCG/Gameplay/Cards/Base/BP_TRCG_Card.BP_TRCG_Card_C|GetData _array_element_3))) false))
  (Development|PrintString "DISCARD STACK :" false)
  (for _array_element_4 (Variables|/Game/TRCG/Gameplay/Cards/Base/BP_TRCG_Stack.BP_TRCG_Stack_C|GetCards (Variables|Default|GetDiscardStack))
    (Development|PrintString (Utilities|String|ToString(Text) (Variables|/Script/TerraCardGame.TrcgCardData|GetCardName (Variables|/Game/TRCG/Gameplay/Cards/Base/BP_TRCG_Card.BP_TRCG_Card_C|GetData _array_element_4))) false))
  (Development|PrintString "HAND :" false)
  (for _array_element_5 (Variables|/Game/TRCG/Gameplay/Cards/Base/BP_TRCG_Hand.BP_TRCG_Hand_C|GetCards (Variables|Default|GetHand))
    (Development|PrintString (Utilities|String|ToString(Text) (Variables|/Script/TerraCardGame.TrcgCardData|GetCardName (Variables|/Game/TRCG/Gameplay/Cards/Base/BP_TRCG_Card.BP_TRCG_Card_C|GetData _array_element_5))) false))
  (Development|PrintString "===================" false)
  (Utilities|IsValid _statmanager
    (:Is%20Valid
      (bind _asbp_trcg_planet_stats_manager (Utilities|Casting|CastToBP_TRCG_PlanetStatsManager _statmanager))
      (Default|CallLogManagedStats _asbp_trcg_planet_stats_manager))))

(event EventBeginPlay
  (EventDispatchers|BindEventtoLogManagedCards (delegate Custom|OnLogManagedCalled))
  (bind _asgi_trcg (Utilities|Casting|CastToGI_TRCG (Class|TrcgActor|GetTrcgGameInstance))
    (:then
      (Variables|/Game/TRCG/General/GI_TRCG.GI_TRCG_C|SetCardManager _asgi_trcg self))
    (:CastFailed
      _))
  (bind _returnvalue (Game|ConstructObjectfromClass "/Game/TRCG/Gameplay/Cards/Base/BP_TRCG_Deck.BP_TRCG_Deck_C" (CallFunction|InitDeck)))
  (Variables|Default|SetDeck _returnvalue)
  (bind _returnvalue_2 (Game|ConstructObjectfromClass "/Game/TRCG/Gameplay/Cards/Base/BP_TRCG_Stack_Action.BP_TRCG_Stack_Action_C"))
  (Variables|Default|SetActionStack _returnvalue_2)
  (bind _returnvalue_3 (Game|ConstructObjectfromClass "/Game/TRCG/Gameplay/Cards/Base/BP_TRCG_Stack_Construction.BP_TRCG_Stack_Construction_C"))
  (Variables|Default|SetConstructionStack _returnvalue_3)
  (bind _returnvalue_4 (Game|ConstructObjectfromClass "/Game/TRCG/Gameplay/Cards/Base/BP_TRCG_Stack_Discard.BP_TRCG_Stack_Discard_C"))
  (Variables|Default|SetDiscardStack _returnvalue_4)
  (bind _returnvalue_5 (Game|ConstructObjectfromClass "/Game/TRCG/Gameplay/Cards/Base/BP_TRCG_Hand.BP_TRCG_Hand_C"))
  (Variables|Default|SetHand _returnvalue_5)
  (bind _returnvalue_6 (Game|ConstructObjectfromClass "/Game/TRCG/Gameplay/Cards/Base/BP_TRCG_Stack_Recycle.BP_TRCG_Stack_Recycle_C"))
  (Variables|Default|SetRecycleStack _returnvalue_6)
  (if (Math|Boolean|ANDBoolean (Utilities|IsValid (Variables|Default|GetDeck)) (Utilities|IsValid (Variables|Default|GetActionStack)) (Utilities|IsValid (Variables|Default|GetConstructionStack)) (Utilities|IsValid (Variables|Default|GetDiscardStack)) (Utilities|IsValid (Variables|Default|GetHand)) (Utilities|IsValid (Variables|Default|GetRecycleStack)))
    (CallFunction|FillStacksfromDeck)
    (bind _asgm_trcg_play (Utilities|Casting|CastToGM_TRCG_Play (Game|GetGameMode)))
    (Default|CallOnCardManagerReady _asgm_trcg_play)
    (else
      (Development|PrintString "ERROR ON INIT" true true "(R=1.000000,G=0.000000,B=0.000000,A=1.000000)"))))

(fn ConstructionScript)

(fn FillStacksfromDeck
  (for _array_element (Variables|/Game/TRCG/Gameplay/Cards/Base/BP_TRCG_Deck.BP_TRCG_Deck_C|GetCards (Variables|Default|GetDeck))
    (bind _asbp_trcg_card_action (Utilities|Casting|CastToBP_TRCG_Card_Action _array_element)
      (:then
        (Default|AddCard (Variables|Default|GetActionStack) _asbp_trcg_card_action))
      (:CastFailed
        (bind _asbp_trcg_card_construction (Utilities|Casting|CastToBP_TRCG_Card_Construction _array_element)
          (:then
            (Default|AddCard (Variables|Default|GetConstructionStack) _asbp_trcg_card_construction))
          (:CastFailed
            (Development|PrintString "ERROR ON FILLCARDSFROMDECK" true true "(R=1.000000,G=0.000000,B=0.000000,A=1.000000)"))))))
  (CallFunction|ShuffleAllStacks)
  (Default|CallLogManagedCards)
  (return))

(fn PickActionCard
  (bind _actionstack (Variables|Default|GetActionStack))
  (bind _cards (Variables|/Game/TRCG/Gameplay/Cards/Base/BP_TRCG_Stack.BP_TRCG_Stack_C|GetCards _actionstack))
  (bind _returnvalue (Utilities|Array|LastIndex _cards))
  (bind _output (Utilities|Array|Get(acopy) _cards _returnvalue))
  (Default|AddCard (Variables|Default|GetHand) _output)
  (Utilities|Array|RemoveItem _cards _output)
  (Default|CallOnHandUpdated)
  (Default|CallLogManagedCards)
  (return))

(fn ShuffleAllStacks
  (Default|Shuffle (Variables|Default|GetActionStack))
  (Default|Shuffle (Variables|Default|GetConstructionStack))
  (return))

(fn PickConstructionCard
  (bind _constructionstack (Variables|Default|GetConstructionStack))
  (bind _cards (Variables|/Game/TRCG/Gameplay/Cards/Base/BP_TRCG_Stack.BP_TRCG_Stack_C|GetCards _constructionstack))
  (bind _output (Utilities|Array|Get(acopy) _cards))
  (Default|AddCard (Variables|Default|GetHand) _output)
  (Utilities|Array|RemoveItem _cards _output)
  (Default|CallOnHandUpdated)
  (Default|CallLogManagedCards)
  (return))

(fn PlayCardfromHand
  (params (CardIndex :type Integer) (Tile :type Trcg%20Tile%20Object%20Reference))
  (bind _hand (Variables|Default|GetHand))
  (bind _cards (Variables|/Game/TRCG/Gameplay/Cards/Base/BP_TRCG_Hand.BP_TRCG_Hand_C|GetCards _hand))
  (bind _output (Utilities|Array|Get(acopy) _cards CardIndex))
  (if (CallFunction|CanbePlayedon Tile _output)
    (Default|UseCard _output (Utilities|Array|FindItem (Variables|/Script/TerraCardGame.TrcgTileManager|GetTiles (Variables|/Script/TerraCardGame.TrcgGameInstance|GetTileManager (Class|TrcgActor|GetTrcgGameInstance))) Tile))
    (Default|AddCard (Variables|Default|GetDiscardStack) _output)
    (Utilities|Array|RemoveItem _cards _output)
    (Default|CallOnHandUpdated)
    (Default|CallLogManagedCards)
    (return)))

(fn DiscardtoDeck
  (if (CallFunction|CanDiscardtoDeck)
    (CallFunction|PurgeStacks false)
    (CallFunction|FillStacksfromDeck)
    (Default|CallLogManagedCards)
    (return)))

(fn PurgeStacks
  (params (PurgeRecycle :type Boolean))
  (Default|Empty (Variables|Default|GetActionStack))
  (Default|Empty (Variables|Default|GetConstructionStack))
  (Default|Empty (Variables|Default|GetDiscardStack))
  (Default|Empty (Variables|Default|GetHand))
  (if PurgeRecycle
    (Default|Empty (Variables|Default|GetRecycleStack)))
  (return))

(fn InitDeck
  (bind _returnvalue (Class|TrcgActor|GetTrcgGameInstance))
  (bind _cardsarray (LocalVariables|GetCardsArray))
  (bind _globaldeck (Variables|/Script/TerraCardGame.TrcgGameInstance|GetGlobalDeck _returnvalue))
  (bind _keys (Utilities|Map|Keys _globaldeck))
  (for _array_element _keys
    (for _index (range 1 (.Value (Utilities|Map|Find _globaldeck _array_element)))
      (switch Utilities|FlowControl|Switch|SwitchonECardType (Variables|/Script/TerraCardGame.TrcgCardData|GetCardType _array_element)
        (:CONSTRUCTION
          (bind _returnvalue_2 (Game|ConstructObjectfromClass "/Game/TRCG/Gameplay/Cards/Base/BP_TRCG_Card_Construction.BP_TRCG_Card_Construction_C" _array_element))
          (Utilities|Array|Add _cardsarray _returnvalue_2))
        (:ACTION
          (bind _returnvalue_3 (Game|ConstructObjectfromClass "/Game/TRCG/Gameplay/Cards/Base/BP_TRCG_Card_Action.BP_TRCG_Card_Action_C" _array_element))
          (Utilities|Array|Add _cardsarray _returnvalue_3)))))
  (return (LocalVariables|GetCardsArray)))

(fn PlayActiveCardfromHand
  (params (Tile :type Trcg%20Tile%20Object%20Reference))
  (if (Utilities|Array|IsValidIndex (Variables|/Game/TRCG/Gameplay/Cards/Base/BP_TRCG_Hand.BP_TRCG_Hand_C|GetCards (Variables|Default|GetHand)) (Variables|Default|GetActiveCardIndex))
    (CallFunction|PlayCardfromHand (Variables|Default|GetActiveCardIndex) Tile)
    (Variables|Default|SetActiveCardIndex -1)))

(fn CanDiscardtoDeck
  (return (and (Utilities|Array|IsEmpty (Variables|/Game/TRCG/Gameplay/Cards/Base/BP_TRCG_Stack.BP_TRCG_Stack_C|GetCards (Variables|Default|GetConstructionStack))) (Utilities|Array|IsEmpty (Variables|/Game/TRCG/Gameplay/Cards/Base/BP_TRCG_Hand.BP_TRCG_Hand_C|GetCards (Variables|Default|GetHand))))))

(fn RecycleActiveCard
  (bind _hand (Variables|Default|GetHand))
  (bind _cards (Variables|/Game/TRCG/Gameplay/Cards/Base/BP_TRCG_Hand.BP_TRCG_Hand_C|GetCards _hand))
  (if (Utilities|Array|IsValidIndex _cards (Variables|Default|GetActiveCardIndex))
    (Utilities|Array|Add (Variables|/Game/TRCG/Gameplay/Cards/Base/BP_TRCG_Stack.BP_TRCG_Stack_C|GetCards (Variables|Default|GetRecycleStack)) (Utilities|Array|Get(acopy) _cards (Variables|Default|GetActiveCardIndex)))
    (Utilities|Array|RemoveItem (Variables|/Game/TRCG/Gameplay/Cards/Base/BP_TRCG_Deck.BP_TRCG_Deck_C|GetCards (Variables|Default|GetDeck)) (Utilities|Array|Get(acopy) _cards (Variables|Default|GetActiveCardIndex)))
    (Utilities|Array|RemoveItem _cards (Utilities|Array|Get(acopy) _cards (Variables|Default|GetActiveCardIndex)))
    (Variables|Default|SetActiveCardIndex -1)
    (Default|CallOnHandUpdated)
    (return)))

(fn GetNewCardfromRecycling
  (params (CardData :type Trcg%20Card%20Data%20Object%20Reference))
  (bind _deck (Variables|Default|GetDeck))
  (bind _cards (Variables|/Game/TRCG/Gameplay/Cards/Base/BP_TRCG_Deck.BP_TRCG_Deck_C|GetCards _deck))
  (switch Utilities|FlowControl|Switch|SwitchonECardType (Variables|/Script/TerraCardGame.TrcgCardData|GetCardType CardData)
    (:CONSTRUCTION
      (bind _returnvalue (Game|ConstructObjectfromClass "/Game/TRCG/Gameplay/Cards/Base/BP_TRCG_Card_Construction.BP_TRCG_Card_Construction_C" CardData))
      (Utilities|Array|Add _cards _returnvalue))
    (:ACTION
      (bind _returnvalue_2 (Game|ConstructObjectfromClass "/Game/TRCG/Gameplay/Cards/Base/BP_TRCG_Card_Action.BP_TRCG_Card_Action_C" CardData))
      (Utilities|Array|Add _cards _returnvalue_2)))
  (Default|Empty (Variables|Default|GetRecycleStack)))

(fn HasActiveCard
  (return (Utilities|Array|IsValidIndex (Variables|/Game/TRCG/Gameplay/Cards/Base/BP_TRCG_Hand.BP_TRCG_Hand_C|GetCards (Variables|Default|GetHand)) (Variables|Default|GetActiveCardIndex))))

(fn GetActiveCard
  (if (CallFunction|HasActiveCard)
    (return (Utilities|Array|Get(acopy) (Variables|/Game/TRCG/Gameplay/Cards/Base/BP_TRCG_Hand.BP_TRCG_Hand_C|GetCards (Variables|Default|GetHand)) (Variables|Default|GetActiveCardIndex)))
    (else
      (return 0))))

(fn CanbePlayedon
  (params (OnTile :type Trcg%20Tile%20Object%20Reference) (Card :type BP%20TRCG%20Card%20Object%20Reference))
  (return (GameplayTags|HasAnyTags (Variables|/Script/TerraCardGame.TrcgCardData|GetTags (Variables|/Game/TRCG/Gameplay/Cards/Base/BP_TRCG_Card.BP_TRCG_Card_C|GetData Card)) (Variables|/Script/TerraCardGame.TrcgTile|GetTileTags OnTile) true)))