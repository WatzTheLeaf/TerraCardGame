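; Tile manager for the TRCG game mode that sets up the tile grid and its play-area bounds on BeginPlay.
; It registers with the game instance, calls GenerateGrid, debug-paints Volcano-tagged tiles red, then notifies GM_TRCG_Play that it is ready.
; GenerateLimit derives the grid center from tile counts and spacing, teleports the player pawn there and spawns a blocking volume sized to the grid.
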(event EventBeginPlay
  (Variables|/Script/TerraCardGame.TrcgGameInstance|SetTileManager (Class|TrcgActor|GetTrcgGameInstance) self)
  (Class|TrcgTileManager|GenerateGrid)
  (CallFunction|DebugMaterialPaint)
  (bind _asgm_trcg_play (Utilities|Casting|CastToGM_TRCG_Play (Game|GetGameMode)))
  (Default|OnTileManagerReadyEvent _asgm_trcg_play)
  (CallFunction|GenerateLimit))

(fn ConstructionScript)

(fn GenerateLimit
  (bind _returnvalue (Game|Player|GetPlayerPawn 0))
  (bind _gridxsize (Variables|Default|GetGridXSize))
  (bind _gridysize (Variables|Default|GetGridYSize))
  (bind _returnvalue_2 (* 1.5e+02 _gridxsize))
  (bind _returnvalue_3 (* _gridysize 1.5e+02))
  (bind _returnvalue_4 (/ _returnvalue_2 2.0))
  (bind _returnvalue_5 (+ _returnvalue_3 -1.5e+02))
  (bind _returnvalue_6 (/ _returnvalue_5 2.0))
  (Rendering|Debug|DrawDebugPoint (Math|Vector|MakeVector _returnvalue_4 _returnvalue_6 1.2e+02) 1e+01 "(R=0.000000,G=0.000000,B=0.000000,A=1.000000)" 6e+01)
  (Transformation|Teleport _returnvalue (Math|Vector|MakeVector _returnvalue_4 _returnvalue_6 1.2e+02) (Transformation|GetActorRotation _returnvalue))
  (Game|SpawnActorfromClass "/Game/TRCG/Gameplay/Misc/BP_TRCG_BlockingVolume.BP_TRCG_BlockingVolume_C" (Math|Transform|MakeTransform (Math|Vector|MakeVector _returnvalue_4 _returnvalue_6 0.0)) "Undefined" "MultiplyWithRoot" 0 (Math|Vector2D|MakeVector2D (+ _returnvalue_6 5e+01) (+ _returnvalue_4 5e+01)) 0)
  (return))

(fn DebugMaterialPaint
  (for _array_element (Variables|Default|GetTiles)
    (if (GameplayTags|HasTag (Variables|/Script/TerraCardGame.TrcgTile|GetTileTags _array_element) "(TagName=\"Tiles.Type.Volcano\")" true)
      (Rendering|Material|SetMaterial (Variables|/Script/TerraCardGame.TrcgTile|GetMesh _array_element) 0 "/Game/TRCG/Assets/Materials/World/Debug/M_DebugTile_Red.M_DebugTile_Red"))))