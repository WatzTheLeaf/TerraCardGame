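; Menu spawn manager for the TRCG card menu, which sets up the camera pawn and card display.
; On BeginPlay it registers itself with the TRCG game instance and waits for an OnHUDReady event.
; When that fires, it spawns a card menu camera, destroys the current player pawn and possesses the camera.
; It then spawns the display card manager that takes grid layout settings for the cards.
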(event Custom|OnHUDReadyEvent
  (bind _returnvalue (Game|SpawnActorfromClass "/Game/TRCG/Gameplay/Misc/BP_CardMenuCam.BP_CardMenuCam_C" (Math|Transform|MakeTransform "0.000000,0.000000,300.000000" "-90.000000,180.000000,180.000000") "Undefined" "MultiplyWithRoot" 0 2e+03 0))
  (Actor|DestroyActor (Game|Player|GetPlayerPawn 0))
  (Pawn|Possess (Game|GetPlayerController 0) _returnvalue)
  (Game|SpawnActorfromClass "/Game/TRCG/Gameplay/Cards/Display/BP_TRCG_DisplayCardManager.BP_TRCG_DisplayCardManager_C" (Math|Transform|MakeTransform "0.000000,0.000000,100.000000") "Undefined" "MultiplyWithRoot" 0 1.5e+02 2e+02 "0.000000,0.000000,100.000000" 3 0))

(event EventBeginPlay
  (bind _asgi_trcg (Utilities|Casting|CastToGI_TRCG (Class|TrcgActor|GetTrcgGameInstance)))
  (Variables|/Game/TRCG/General/GI_TRCG.GI_TRCG_C|SetMenuSpawnManager _asgi_trcg self)
  (EventDispatchers|BindEventtoOnHUDReady (delegate Custom|OnHUDReadyEvent)))

(fn ConstructionScript)