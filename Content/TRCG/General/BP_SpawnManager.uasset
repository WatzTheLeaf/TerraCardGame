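; Bootstrap actor for the TRCG game that registers itself with GI_TRCG and spawns the core managers in a fixed order.
; BeginPlay binds ready events, then spawns the card manager; its readiness triggers a 4x6 tile manager, whose readiness triggers the planet stats manager.
; Once stats are ready, it destroys the player pawn and spawns BP_GameCam, so startup is event-chained rather than timed.
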(event Custom|OnCardManagerReadyEvent
  (Game|SpawnActorfromClass "/Game/TRCG/Gameplay/World/BP_TRCG_TileManager.BP_TRCG_TileManager_C" (Math|Transform|MakeTransform "0, 0, 0") "Undefined" "MultiplyWithRoot" 0 4 6 0))

(event Custom|OnTileManagerReadyEvent
  (Game|SpawnActorfromClass "/Game/TRCG/Gameplay/Stats/BP_TRCG_PlanetStatsManager.BP_TRCG_PlanetStatsManager_C" (Math|Transform|MakeTransform "0, 0, 0") "Undefined" "MultiplyWithRoot" 0 0))

(event Custom|OnStatManagerReadyEvent
  (Actor|DestroyActor (Game|Player|GetPlayerPawn 0))
  (Game|SpawnActorfromClass "/Game/TRCG/Gameplay/Misc/BP_GameCam.BP_GameCam_C" (Math|Transform|MakeTransform "0.000000,0.000000,100.000000") "Undefined" "MultiplyWithRoot" 0 1e+03 2.0 6e+02 0))

(event EventBeginPlay
  (EventDispatchers|BindEventtoOnCardManagerReady (delegate Custom|OnCardManagerReadyEvent))
  (EventDispatchers|BindEventtoOnTileManagerReady (delegate Custom|OnTileManagerReadyEvent))
  (EventDispatchers|BindEventtoOnStatManagerReady (delegate Custom|OnStatManagerReadyEvent))
  (bind _asgi_trcg (Utilities|Casting|CastToGI_TRCG (Class|TrcgActor|GetTrcgGameInstance)))
  (Variables|/Game/TRCG/General/GI_TRCG.GI_TRCG_C|SetSpawnManager _asgi_trcg self)
  (Game|SpawnActorfromClass "/Game/TRCG/Gameplay/Cards/BP_TRCG_CardManager.BP_TRCG_CardManager_C" (Math|Transform|MakeTransform "0, 0, 0") "Undefined" "MultiplyWithRoot" 0 0))

(fn ConstructionScript)