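; Spawn manager for the TRCG game that creates the core managers in sequence and registers itself with the game instance.
; Ready events chain the setup: HUD ready spawns the card manager, which leads to the tile manager with its grid size, then the planet stats manager.
; Once stats are ready, it spawns the game camera, replaces and destroys the player pawn, and signals readiness to create the HUD.
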(event Custom|OnHUDReadyEvent
  (Game|SpawnActorfromClass "/Game/TRCG/Gameplay/Cards/BP_TRCG_CardManager.BP_TRCG_CardManager_C" (Math|Transform|MakeTransform "0, 0, 0") "Undefined" "MultiplyWithRoot" 0 0))

(event Custom|OnCardManagerReadyEvent
  (Game|SpawnActorfromClass "/Game/TRCG/Gameplay/World/BP_TRCG_TileManager.BP_TRCG_TileManager_C" (Math|Transform|MakeTransform "0, 0, 0") "Undefined" "MultiplyWithRoot" 0 4 6 0))

(event Custom|OnTileManagerReadyEvent
  (Game|SpawnActorfromClass "/Game/TRCG/Gameplay/Stats/BP_TRCG_PlanetStatsManager.BP_TRCG_PlanetStatsManager_C" (Math|Transform|MakeTransform "0, 0, 0") "Undefined" "MultiplyWithRoot" 0 0))

(event Custom|OnStatManagerReadyEvent
  (bind _returnvalue (Game|SpawnActorfromClass "/Game/TRCG/Gameplay/Misc/BP_GameCam.BP_GameCam_C" (Math|Transform|MakeTransform "0.000000,0.000000,120.000000") "Undefined" "MultiplyWithRoot" 0 1e+03 1e+02 6e+02 0))
  (Actor|DestroyActor (Game|Player|GetPlayerPawn 0))
  (Pawn|Possess (Game|GetPlayerController 0) _returnvalue)
  (Default|CallOnReadytoCreateHUD _returnvalue))

(event EventBeginPlay
  (EventDispatchers|BindEventtoOnCardManagerReady (delegate Custom|OnCardManagerReadyEvent))
  (EventDispatchers|BindEventtoOnTileManagerReady (delegate Custom|OnTileManagerReadyEvent))
  (EventDispatchers|BindEventtoOnStatManagerReady (delegate Custom|OnStatManagerReadyEvent))
  (EventDispatchers|BindEventtoOnHUDReady (delegate Custom|OnHUDReadyEvent))
  (bind _asgi_trcg (Utilities|Casting|CastToGI_TRCG (Class|TrcgActor|GetTrcgGameInstance)))
  (Variables|/Game/TRCG/General/GI_TRCG.GI_TRCG_C|SetGameSpawnManager _asgi_trcg self))

(fn ConstructionScript)